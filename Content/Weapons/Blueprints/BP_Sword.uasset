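; Sword weapon that damages other third-person characters and snaps back onto the character it started attached to.
; Shortly after BeginPlay it caches that parent character and its attach socket.
; Blade overlaps apply point damage to other characters and print the result.
; Overlaps with its own character, when GotSword is false, disable physics, reattach it to the mesh socket and set the flag.
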(event `self.ReceiveBeginPlay`
  (`KismetSystemLibrary.Delay` 0.2)
  (set `self.MyChar` (`self.GetAttachParentActor` (`ActorComponent.GetOwner` (`self.Sword`))))
  (set `self.Socket` (`self.GetAttachParentSocketName`)))

(event `self.Blade.OnComponentBeginOverlap`
  (params (OverlappedComponent :type "PrimitiveComponent Object Reference") (OtherActor :type "Actor Object Reference") (OtherComp :type "PrimitiveComponent Object Reference") (OtherBodyIndex :type Integer) (bFromSweep :type Boolean) (SweepResult :type "HitResult Structure (by ref)"))
  (bind _asbp_third_person_character (cast `/Game/Characters/Blueprints/BP_ThirdPersonCharacter` OtherActor))
  (if (not (== (`self.MyChar`) _asbp_third_person_character))
    (bind _returnvalue (`GameplayStatics.ApplyPointDamage` _asbp_third_person_character (`self.Damage`) (`KismetMathLibrary.SelectVector` (0.0 0.0 0.0) (0.0 0.0 0.0) bFromSweep) SweepResult))
    (`KismetSystemLibrary.PrintText` (`KismetTextLibrary.Conv_DoubleToText` _returnvalue "HalfToEven"))))

(event `self.Sword.OnComponentBeginOverlap`
  (params (OverlappedComponent :type "PrimitiveComponent Object Reference") (OtherActor :type "Actor Object Reference") (OtherComp :type "PrimitiveComponent Object Reference") (OtherBodyIndex :type Integer) (bFromSweep :type Boolean) (SweepResult :type "HitResult Structure (by ref)"))
  (bind _asbp_third_person_character (cast `/Game/Characters/Blueprints/BP_ThirdPersonCharacter` OtherActor))
  (if (== (`self.MyChar`) _asbp_third_person_character)
    (if (not (`/Game/Characters/Blueprints/BP_ThirdPersonCharacter.GotSword?` _asbp_third_person_character))
      (`PrimitiveComponent.SetSimulatePhysics` (`self.Sword`) false)
      (`self.K2_AttachToComponent` (`Character.Mesh` _asbp_third_person_character) (`self.Socket`) "SnapToTarget" "SnapToTarget" "SnapToTarget")
      (set `/Game/Characters/Blueprints/BP_ThirdPersonCharacter.GotSword?` true _asbp_third_person_character))))

(fn `UserConstructionScript`)