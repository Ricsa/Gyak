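; BP_AI_Character is an AI character Blueprint that handles taking damage and dying.
; AnyDamage passes damage to TakeDamage, which subtracts it from Health, then prints a debug message.
; When IsDead finds Health at or below zero, TakeDamage destroys attached actors and the character, then calls UnPossess on its controller.
; An unconnected DetachFromActor node remains in TakeDamage and never runs.
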(event `self.ReceiveAnyDamage`
  (params (Damage :type "Float (single-precision)") (DamageType :type "DamageType Object Reference") (InstigatedBy :type "Controller Object Reference") (DamageCauser :type "Actor Object Reference"))
  (`self.Take Damage` Damage)
  (`KismetSystemLibrary.PrintString` "Took Damage"))

(fn `Is Dead`
  (returns (Dead :type Boolean))
  (return (<= (`self.Health`) 0.0)))

(fn `Take Damage`
  (params (Damage :type "Float (double-precision)"))
  (set `self.Health` (- (`self.Health`) Damage))
  (if (`self.Is Dead`)
    (`self.K2_DestroyActor` (`self.GetAttachedActors`))
    (`self.K2_DestroyActor`)
    (`Controller.UnPossess` (`self.GetController`))))

(fn `UserConstructionScript`)