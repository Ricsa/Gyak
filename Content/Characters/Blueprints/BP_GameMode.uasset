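; Game mode Blueprint that spawns BP_ThirdPersonCharacter instances at a fixed location, apparently as enemies, while the live enemy count is low.
; BeginPlay resets LiveEnemies to zero, and a Delay on Tick throttles the count check to roughly every two seconds.
; Each spawn ignores collisions, passes GetAIController as owner and overwrites CharRef.
; LiveEnemies is not incremented here, so spawning repeats unless other code updates it.
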(event `self.ReceiveBeginPlay`
  (set `self.LiveEnemies` 0))

(event `self.ReceiveTick`
  (params (DeltaSeconds :type "Float (single-precision)"))
  (`KismetSystemLibrary.Delay` 2.0)
  (if (<= (`KismetMathLibrary.Conv_IntToDouble` (`self.LiveEnemies`)) 1.0)
    (bind _returnvalue (`|SpawnActorFromClass` "/Game/Characters/Blueprints/BP_ThirdPersonCharacter.BP_ThirdPersonCharacter_C" (`KismetMathLibrary.MakeTransform` (420.0 60.0 453.0) (struct :`Yaw` 180.0)) "AlwaysSpawn" "OverrideRootScale" (`AIBlueprintHelperLibrary.GetAIController` null) null))
    (set `self.CharRef` _returnvalue)))

(fn `UserConstructionScript`)